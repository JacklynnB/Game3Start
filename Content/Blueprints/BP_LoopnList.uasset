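; BP_LoopnList is a test actor that prints randomly colored "KEYGEN" debug messages in an endless loop from BeginPlay.
; LoopdeLoop prints and increments a counter, waits on a Delay, fires keygen, then calls itself again.
; Keygen shuffles TextCol but uses it only for the line count, drawing each color from an inline rainbow array.
; It finishes by printing a random index from that palette.
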(event `LoopdeLoop`
  (`KismetSystemLibrary.PrintString` (`KismetStringLibrary.Concat_StrStr` "KEYGEN:: " (`KismetStringLibrary.Conv_IntToString` (`self.DelayloopCounter`))))
  (`/Engine/EditorBlueprintResources/StandardMacros.IncrementInt` (`self.DelayloopCounter`)
    (:`  `
      (`KismetSystemLibrary.Delay` 1.0)
      (`self.keygen`)
      (`self.LoopdeLoop`))))

(event `self.ReceiveBeginPlay`
  (`KismetSystemLibrary.PrintString` "Loop and List is active")
  (`self.LoopdeLoop`))

(event `keygen`
  (bind _textcol (`self.TextCol`))
  (bind (_outitem _outindex) (`KismetArrayLibrary.Array_Random` (`|MakeArray` (struct :`R` 1.0 :`A` 1.0) (struct :`R` 1.0 :`G` 0.5 :`A` 1.0) (struct :`R` 1.0 :`G` 1.0 :`A` 1.0) (struct :`G` 1.0 :`A` 1.0) (struct :`B` 1.0 :`A` 1.0) (struct :`R` 0.5 :`B` 1.0 :`A` 1.0) (struct :`R` 1.0 :`B` 0.5 :`A` 1.0) :!type "LinearColor Structure")))
  (`KismetArrayLibrary.Array_Shuffle` _textcol)
  (for _ _textcol
    (`KismetSystemLibrary.PrintString` "-=:KEYGEN:=-" true true _outitem))
  (`KismetSystemLibrary.PrintString` (`KismetStringLibrary.Concat_StrStr` "" (`KismetStringLibrary.Conv_IntToString` _outindex))))

(fn `UserConstructionScript`)