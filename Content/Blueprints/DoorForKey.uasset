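; DoorForKey is a locked door that opens when a BP_ThirdPersonCharacter holding at least one key enters its Sphere trigger.
; The overlap deducts one key from the character and plays the DoorOpen timeline, which lerps the DORE component's relative Z to lower the door.
; Without a key it prints a red locked message.
; No opened state is tracked, so each later overlap with keys deducts another.
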(event `self.ReceiveBeginPlay`
  (`KismetSystemLibrary.PrintString` "There's a Door round these parts..."))

(event `self.Sphere.OnComponentBeginOverlap`
  (params (OverlappedComponent :type "PrimitiveComponent Object Reference") (OtherActor :type "Actor Object Reference") (OtherComp :type "PrimitiveComponent Object Reference") (OtherBodyIndex :type Integer) (bFromSweep :type Boolean) (SweepResult :type "HitResult Structure (by ref)"))
  (bind _dore (`self.DORE`))
  (bind (_relativelocation_x _relativelocation_y) (`KismetMathLibrary.BreakVector` (`SceneComponent.RelativeLocation` _dore)))
  (bind _asbp_third_person_character (cast `/Game/ThirdPerson/Blueprints/BP_ThirdPersonCharacter` OtherActor))
  (bind _keys (`/Game/ThirdPerson/Blueprints/BP_ThirdPersonCharacter.Keys` _asbp_third_person_character))
  (if (> _keys 0)
    (`KismetSystemLibrary.PrintString` "DOOR UNLOCKED... OPENING...")
    (set `/Game/ThirdPerson/Blueprints/BP_ThirdPersonCharacter.Keys` (+ _keys -1) _asbp_third_person_character)
    (bind (_direction _newtrack_0) (`Timeline|Door Open`)
      (:`Update`
        (`SceneComponent.K2_SetRelativeLocation` _dore (`KismetMathLibrary.MakeVector` _relativelocation_x _relativelocation_y (`KismetMathLibrary.Lerp` 100.0 -99.0 _newtrack_0)) false false)))
    (else
      (`KismetSystemLibrary.PrintString` "You need a key, this door's locked! :(" true true (struct :`R` 1.0 :`A` 1.0)))))

(fn `UserConstructionScript`)