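; BP_ElementalBarrier is a barrier actor with one elemental type that only characters immune to that element can pass safely.
; On BeginPlay it sets its text render label to name the element: fire, water, earth, poison or wind.
; Cube overlap compares the type with the ThirdPersonCharacter's ElementalImmunity.
; A mismatch prints a placeholder message and quits the game after a short delay, with no damage or respawn step.
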(event `self.ReceiveBeginPlay`
  (switch `/Game/Blueprints/ElementalType` (`self.Elemental type`)
    (:`NewEnumerator1`
      (`TextRenderComponent.K2_SetText` (`self.TextRender`) "Barrier of FIRE"))
    (:`NewEnumerator2`
      (`TextRenderComponent.K2_SetText` (`self.TextRender`) "Barrier of WATER"))
    (:`NewEnumerator3`
      (`TextRenderComponent.K2_SetText` (`self.TextRender`) "Barrier of EARTH"))
    (:`NewEnumerator4`
      (`TextRenderComponent.K2_SetText` (`self.TextRender`) "Barrier of POISON"))
    (:`NewEnumerator5`
      (`TextRenderComponent.K2_SetText` (`self.TextRender`) "Barrier of WIND"))))

(event `self.Cube.OnComponentBeginOverlap`
  (params (OverlappedComponent :type "PrimitiveComponent Object Reference") (OtherActor :type "Actor Object Reference") (OtherComp :type "PrimitiveComponent Object Reference") (OtherBodyIndex :type Integer) (bFromSweep :type Boolean) (SweepResult :type "HitResult Structure (by ref)"))
  (bind _asbp_third_person_character (cast `/Game/ThirdPerson/Blueprints/BP_ThirdPersonCharacter` OtherActor))
  (if (not (`|EnumEquality` (`self.Elemental type`) (`/Game/ThirdPerson/Blueprints/BP_ThirdPersonCharacter.Elemental Immunity` _asbp_third_person_character)))
    (`KismetSystemLibrary.PrintText` "Hello")
    (`KismetSystemLibrary.Delay` 0.2)
    (`KismetSystemLibrary.QuitGame` null "Quit" true)))

(fn `UserConstructionScript`)